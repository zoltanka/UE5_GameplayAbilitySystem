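; BP_Tile_1x1x1 is a tile actor that bobs up and down around the position where it begins play.
; BeginPlay stores the starting location, and Tick accumulates elapsed time in Delta.
; Each frame, a sine of that time, scaled by a fixed amplitude, offsets the stored Z while X and Y stay at their starting values.
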(event `self.ReceiveBeginPlay`
  (set `self.StartingLocaton` (`self.K2_GetActorLocation`)))

(event `self.ReceiveTick`
  (params (DeltaSeconds :type "Float (single-precision)"))
  (bind (_startinglocaton_x _startinglocaton_y _startinglocaton_z) (`KismetMathLibrary.BreakVector` (`self.StartingLocaton`)))
  (bind _output_get (set `self.Delta` (+ DeltaSeconds (`self.Delta`))))
  (`self.K2_SetActorLocation` (`KismetMathLibrary.MakeVector` _startinglocaton_x _startinglocaton_y (+ _startinglocaton_z (* (`KismetMathLibrary.Sin` _output_get) 15.0)))))

(fn `UserConstructionScript`)